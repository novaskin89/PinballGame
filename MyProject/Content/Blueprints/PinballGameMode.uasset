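; Pinball game mode that runs the session from main menu through play to the win or lose screen.
; ResetGame restores class defaults, creates the HUD and spawns a ball at the plunger; destroyed balls respawn after a delay until none remain.
; EndGame and WinGame compare score to the lowest saved high score, though both branches open the same Lose or Win menu.
; AddScore applies the multiplier; GetGameSaveData caches the loaded or new save.
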(event `ResetGame`
  (bind (_score _multiplier _ballsremaining _tiltcount) (defaults `/Game/Blueprints/PinballGameMode` "PinballGameMode_C"))
  (bind _aspinball_player_controller (cast `/Game/Blueprints/Pinball_Player_controller` (`GameplayStatics.GetPlayerController` 0) :!pure true))
  ;[1 1 1] Reset Game
  (set `self.Win?` false)
  (`self.EnableInput` (cast `/Game/Blueprints/Pinball_Player_controller` (`GameplayStatics.GetPlayerController` 0) :!pure true) null)
  (set `self.Score` _score)
  (set `self.Multiplier` _multiplier)
  (set `self.BallsRemaining` _ballsremaining)
  (set `self.TiltCount` _tiltcount)
  (`self.SpawnBall`)
  (`/Game/Blueprints/Pinball_Player_controller.CreatePlayerHUD` _aspinball_player_controller)
  (set `PlayerController.bShowMouseCursor` false _aspinball_player_controller)
  (`self.OnGameReset`))

(event `self.ReceiveBeginPlay`
  (`self.DisableInput` (cast `/Game/Blueprints/Pinball_Player_controller` (`GameplayStatics.GetPlayerController` 0) :!pure true) null)
  (`self.CreateMainMenu`)
  (`GameplayStatics.PlaySound2D` "/Game/Sounds/victoryMusic_loop_01_01.victoryMusic_loop_01_01" 0.2))

(event `SpawnBall`
  (bind _outactors (`GameplayStatics.GetAllActorsOfClass` "/Game/Blueprints/BP_Plunger.BP_Plunger_C"))
  (bind _returnvalue (`|SpawnActorFromClass` "/Game/Blueprints/BP_Ball.BP_Ball_C" (`KismetMathLibrary.MakeTransform` (`/Game/Blueprints/BP_Plunger.GetBallSpawnLocation` (`|GetArrayItem` _outactors))) "Undefined" "OverrideRootScale"))
  (add `self.OnDestroyed` _returnvalue (delegate `OnBallDestroyed`)))

(event `OnBallDestroyed` :!signature `self.OnDestroyed`
  (params (DestroyedActor :type "Actor Object Reference"))
  (if (`self.Win?`)
    _
    (elif (> (`self.BallsRemaining`) 0)
      (`KismetSystemLibrary.Delay` 1.5)
      (`self.SpawnBall`)
      (`/Engine/EditorBlueprintResources/StandardMacros.DecrementInt` (`self.BallsRemaining`))
      (else
        (`self.EndGame`)))))

(event `EndGame`
  (bind _aspinball_player_controller (cast `/Game/Blueprints/Pinball_Player_controller` (`GameplayStatics.GetPlayerController` 0) :!pure true))
  (`self.DisableInput` _aspinball_player_controller null)
  (set `PlayerController.bShowMouseCursor` true _aspinball_player_controller)
  (bind _currentsaveobject (`self.GetGameSaveData`))
  (if (<= (`KismetArrayLibrary.Array_Length` (`/Game/Blueprints/HighScoreSave.SaveStruct` _currentsaveobject)) 3)
    _
    (else
      _))
  (bind _lowestscorestruct (`/Game/Blueprints/HighScoreSave.DetermineLowestScoreValue` _currentsaveobject))
  (if (< (`.Score_7_2435521C45FFA07F11D27DB46D00B598` (break `/Game/Blueprints/HighScoreStruct` _lowestscorestruct)) (`self.Score`))
    (`self.CreateHighScoreList 1`)
    (else
      (bind _returnvalue (`|CreateWidget` "/Game/Widget/LoseMenu.LoseMenu_C"))
      (`UserWidget.AddToViewport` _returnvalue 0))))

(event `CreateHighScoreList 1`
  (bind _aspinball_player_controller (cast `/Game/Blueprints/Pinball_Player_controller` (`GameplayStatics.GetPlayerController` 0) :!pure true))
  (bind _returnvalue (`|CreateWidget` "/Game/Widget/LoseMenu.LoseMenu_C" _aspinball_player_controller))
  (`UserWidget.AddToViewport` _returnvalue 0)
  (set `PlayerController.bShowMouseCursor` true _aspinball_player_controller))

(event `CreateMainMenu`
  (bind _aspinball_player_controller (cast `/Game/Blueprints/Pinball_Player_controller` (`GameplayStatics.GetPlayerController` 0) :!pure true))
  (`self.GetGameSaveData`)
  (`WidgetLayoutLibrary.RemoveAllWidgets`)
  (bind _returnvalue (`|CreateWidget` "/Game/Widget/MainMenu.MainMenu_C" _aspinball_player_controller))
  (`UserWidget.AddToViewport` _returnvalue 0)
  (set `PlayerController.bShowMouseCursor` true _aspinball_player_controller))

(event `WinGame`
  (bind _aspinball_player_controller (cast `/Game/Blueprints/Pinball_Player_controller` (`GameplayStatics.GetPlayerController` 0) :!pure true))
  (set `self.Win?` true)
  (`/Engine/EditorBlueprintResources/StandardMacros.IncrementInt` (`self.BallsRemaining`)
    (:`  `
      (bind _outactors (`GameplayStatics.GetAllActorsOfClass` "/Game/Blueprints/BP_Plunger.BP_Plunger_C"))
      (for _array_element _outactors
        (`self.K2_DestroyActor` _array_element)
        (`self.DisableInput` _aspinball_player_controller null)
        (set `PlayerController.bShowMouseCursor` true _aspinball_player_controller)
        (bind _currentsaveobject (`self.GetGameSaveData`))
        (if (<= (`KismetArrayLibrary.Array_Length` (`/Game/Blueprints/HighScoreSave.SaveStruct` _currentsaveobject)) 3)
          _
          (else
            _))
        (bind _lowestscorestruct (`/Game/Blueprints/HighScoreSave.DetermineLowestScoreValue` _currentsaveobject))
        (if (< (`.Score_7_2435521C45FFA07F11D27DB46D00B598` (break `/Game/Blueprints/HighScoreStruct` _lowestscorestruct)) (`self.Score`))
          (`self.CreateHighScoreList2`)
          (else
            (bind _returnvalue (`|CreateWidget` "/Game/Widget/WinMenu.WinMenu_C"))
            (`UserWidget.AddToViewport` _returnvalue 0)))))))

(event `CreateHighScoreList2`
  (bind _aspinball_player_controller (cast `/Game/Blueprints/Pinball_Player_controller` (`GameplayStatics.GetPlayerController` 0) :!pure true))
  (bind _returnvalue (`|CreateWidget` "/Game/Widget/WinMenu.WinMenu_C" _aspinball_player_controller))
  (`UserWidget.AddToViewport` _returnvalue 0)
  (set `PlayerController.bShowMouseCursor` true _aspinball_player_controller))

(fn `AddScore`
  (params (PointsToAdd :type "Float (double-precision)"))
  (returns (NewScore :type "Float (double-precision)"))
  (bind _output_get (set `self.Score` (+ (* PointsToAdd (`self.Multiplier`)) (`self.Score`))))
  (return _output_get))

(fn `GetGameSaveData`
  (returns (CurrentSaveObject :type "/Game/Blueprints/HighScoreSave Object Reference"))
  (bind _currentsaveobject (`self.CurrentSaveObject`)
    (:`then`
      (return _currentsaveobject))
    (:`else`
      (bind _returnvalue (`GameplayStatics.DoesSaveGameExist` (`self.HighScoreSaveName`)))
      (if _returnvalue
        (bind _returnvalue_2 (`GameplayStatics.LoadGameFromSlot` (`self.HighScoreSaveName`)))
        (bind _ashigh_score_save (cast `/Game/Blueprints/HighScoreSave` _returnvalue_2)
          (:`then`
            (`/Game/Blueprints/HighScoreSave.SortSaveData` _ashigh_score_save)
            (bind _output_get (set `self.CurrentSaveObject` _ashigh_score_save))
            (return _output_get))
          (:`CastFailed`
            (return _ashigh_score_save)))
        (else
          (bind _returnvalue_3 (`GameplayStatics.CreateSaveGameObject` "/Game/Blueprints/HighScoreSave.HighScoreSave_C"))
          (bind _output_get_2 (set `self.CurrentSaveObject` _returnvalue_3))
          (return _output_get_2))))))

(fn `UserConstructionScript`)