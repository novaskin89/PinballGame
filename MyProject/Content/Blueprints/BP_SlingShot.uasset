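; Pinball slingshot bumper that scores points and kicks the ball away when a BP_Ball overlaps it.
; On overlap it adds score through PinballGameMode, applies a mass-independent impulse against the capsule's forward vector and plays a sound at world origin.
; The SlingBounce timeline then animates the bounce by driving the PercentOut parameter on a dynamic mesh material created in the construction script.
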(event `self.ReceiveActorBeginOverlap`
  (params (OtherActor :type "Actor Object Reference"))
  (bind _asbp_ball (cast `/Game/Blueprints/BP_Ball` OtherActor))
  (bind _aspinball_game_mode (cast `/Game/Blueprints/PinballGameMode` (`GameplayStatics.GetGameMode`))
    (:`then`
      (`/Game/Blueprints/PinballGameMode.AddScore` _aspinball_game_mode 200.0))
    (:`CastFailed`
      _))
  (`PrimitiveComponent.AddImpulse` (`/Game/Blueprints/BP_Ball.Ball` _asbp_ball) (* (`SceneComponent.GetForwardVector` (`self.Capsule`)) -2500.0) "None" true)
  (`GameplayStatics.PlaySoundAtLocation` "/Game/Sounds/Arcade_Enemy_Death_03_m1.Arcade_Enemy_Death_03_m1")
  (bind (_direction _bounce) (`Timeline|SlingBounce` :!via `PlayFromStart`)
    (:`Update`
      (bind _asmaterial_instance_dynamic (cast `MaterialInstanceDynamic` (`PrimitiveComponent.GetMaterial` (`self.StaticMesh`) 2)))
      (`MaterialInstanceDynamic.SetScalarParameterValue` _asmaterial_instance_dynamic "PercentOut" _bounce))))

(event `self.Capsule.OnComponentBeginOverlap`
  (params (OverlappedComponent :type "PrimitiveComponent Object Reference") (OtherActor :type "Actor Object Reference") (OtherComp :type "PrimitiveComponent Object Reference") (OtherBodyIndex :type Integer) (bFromSweep :type Boolean) (SweepResult :type "HitResult Structure (by ref)")))

(fn `UserConstructionScript`
  (`PrimitiveComponent.CreateDynamicMaterialInstance` (`self.StaticMesh`) 2 null))